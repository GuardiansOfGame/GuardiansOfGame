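; BlockMonster_BP is a monster that fires at the player and dies when a weapon damages it.
; When a GOGCharacter enters its Sphere, it spawns a Bullet at its own transform and destroys it after one second.
; Any damage caused by a Weapon spawns an explosion emitter and destroys the monster immediately, with no health check.
; Tick reassigns the AI controller class to MonsterAI every frame.
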(event OnComponentBeginOverlap(Sphere)
  (params (OverlappedComponent :type Primitive%20Component%20Object%20Reference) (OtherActor :type Actor%20Object%20Reference) (OtherComp :type Primitive%20Component%20Object%20Reference) (OtherBodyIndex :type Integer) (bFromSweep :type Boolean) (SweepResult :type Hit%20Result%20Structure%20%28by%20ref%29))
  (Utilities|Casting|CastToGOGCharacter OtherActor)
  (bind _returnvalue (Game|SpawnActorfromClass "/Game/CustomContent/MonsterJIna/Bullet.Bullet_C" (Transformation|GetActorTransform) "Undefined" 0 0))
  (Utilities|FlowControl|Delay 1.0)
  (Actor|DestroyActor _returnvalue))

(event EventBeginPlay)

(event Collision|EventActorBeginOverlap
  (params (OtherActor :type Actor%20Object%20Reference)))

(event EventTick
  (params (DeltaSeconds :type Float%20%28single-precision%29))
  (Variables|Default|SetAIControllerClass "/Script/GuardiansOfGame.MonsterAI"))

(event Game|Damage|EventAnyDamage
  (params (Damage :type Float%20%28single-precision%29) (DamageType :type Damage%20Type%20Object%20Reference) (InstigatedBy :type Controller%20Object%20Reference) (DamageCauser :type Actor%20Object%20Reference))
  (Utilities|Casting|CastToWeapon DamageCauser)
  (Effects|SpawnEmitteratLocation "/Game/StarterContent/Particles/P_Explosion.P_Explosion" (Transformation|GetActorLocation))
  (Actor|DestroyActor))

(fn ConstructionScript)