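; Boss enemy that reacts to GOGCharacter overlapping its sphere.
; A FlipFlop alternates overlaps between a boss attack (camera shake, printed player HP loss, BlockMonster_BP spawn) and a hit on the boss with an attacked animation.
; BossHP counts hits upward; an overlap once it equals three plays the death animation and destroys the actor after a delay.
; Player damage is only printed, not applied.
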(event OnComponentBeginOverlap(Sphere)
  (params (OverlappedComponent :type Primitive%20Component%20Object%20Reference) (OtherActor :type Actor%20Object%20Reference) (OtherComp :type Primitive%20Component%20Object%20Reference) (OtherBodyIndex :type Integer) (bFromSweep :type Boolean) (SweepResult :type Hit%20Result%20Structure%20%28by%20ref%29))
  (Utilities|Casting|CastToGOGCharacter OtherActor)
  (if (== (Variables|Default|GetBossHP) 3)
    (Utilities|FlowControl|DoOnce false
      (:Completed
        (Components|Animation|PlayAnimation (Variables|Character|GetMesh) "/Game/CustomContent/Monster/Boss/boss_Anim_Die.boss_Anim_Die" false)
        (Utilities|FlowControl|Delay 2.5)
        (Actor|DestroyActor)))
    (else
      (Utilities|FlowControl|FlipFlop
        (:A
          (Class|MatineeCameraShake|StartMatineeCameraShake (Variables|/Script/Engine.PlayerController|GetPlayerCameraManager (Game|GetPlayerController 0)) "/Game/CustomContent/Monster/Boss/MyShake.MyShake_C" 1.0 "CameraLocal" "0, 0, 0")
          (Development|PrintString "HP -10")
          (Game|SpawnActorfromClass "/Game/CustomContent/Monster_BP/BlockMonster_BP.BlockMonster_BP_C" (Transformation|GetActorTransform) "AdjustIfPossibleButAlwaysSpawn" 0 0))
        (:B
          (Utilities|FlowControl|DoOnce false :!label _label
            (:Completed
              (Components|Animation|PlayAnimation (Variables|Character|GetMesh) "/Game/CustomContent/Monster/Boss/boss_Anim_attacked.boss_Anim_attacked" false)
              (Development|PrintString "Boss -10")
              (bind _result (Math|Integer|IncrementInt (Variables|Default|GetBossHP))
                (:%20%20
                  (Variables|Default|SetBossHP _result)
                  (goto _label Reset))))))))))

(event EventBeginPlay)

(event Collision|EventActorBeginOverlap
  (params (OtherActor :type Actor%20Object%20Reference)))

(event EventTick
  (params (DeltaSeconds :type Float%20%28single-precision%29)))

(fn ConstructionScript)